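; Procedural inverted-staircase block piece that builds a stepped wall of stone instances in its construction script.
; A nested loop over the X and Z counts adds instances only where the row index is at least the column index, spacing them by mesh bounds.
; A seeded stream, two random indices and three custom data floats are set up but never used in placement.
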(event EventBeginPlay)

(fn ConstructionScript
  (bind _cube (Variables|Default|Getcube))
  (bind (_min _max) (Components|StaticMesh|GetLocalBounds _cube))
  (Math|Random|SetRandomStreamSeed (Variables|Default|GetStream) (Variables|Default|GetSeed))
  (LocalVariables|SetRandX (Math|Random|RandomIntegerinRange 0 (- (Variables|Default|GetX) 1)))
  (LocalVariables|SetRandY (Math|Random|RandomIntegerinRange 0 (- (Variables|Default|GetZ) 1)))
  (Class|InstancedStaticMeshComponent|SetNumCustomDataFloats (Variables|Default|Getcube) 3)
  ;[1 1 1] set static mesh et material
  (Components|StaticMesh|SetStaticMesh (Variables|Default|Getcube) (Variables|Default|GetSM_Stone))
  (LocalVariables|Setcenter (- _max _min))
  (for _index (range 0 (- (Variables|Default|GetZ) 1))
    (bind _output_get (LocalVariables|SetZindex _index))
    (for _index_2 (range 0 (- (Variables|Default|GetX) 1))
      (bind _output_get_2 (LocalVariables|SetIndexX _index_2))
      (if (>= _output_get_2 _output_get)
        (Components|InstancedStaticMesh|AddInstance (Variables|Default|Getcube) (Math|Transform|MakeTransform (Math|Vector|MakeVector (* (.x (LocalVariables|Getcenter)) (LocalVariables|GetZindex)) 0.0 (+ (* (.z (LocalVariables|Getcenter)) (LocalVariables|GetIndexX)) 5e+01)) "0, 0, 0" "1.000000,1.000000,1.000000") false)))))