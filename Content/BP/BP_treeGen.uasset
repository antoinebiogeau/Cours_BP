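; Procedural tree generator Blueprint that builds a seeded, jittered random-walk spline in its construction script, with no mesh placement.
; Each step rotates CurrentDir by random roll and pitch, normalizes it, scales it by random per-axis distances and offsets it from CurrentLoc.
; That pure expression re-rolls for the spline point, CurrentLoc and CurrentDir separately, so they differ, and CurrentDir receives a position rather than an offset.
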(event EventBeginPlay)

(event Collision|EventActorBeginOverlap
  (params (OtherActor :type Actor%20Object%20Reference)))

(event EventTick
  (params (DeltaSeconds :type Float%20%28single-precision%29)))

(fn ConstructionScript
  (bind _stream (LocalVariables|GetStream))
  (bind _maxdist (Variables|Default|GetMaxDist))
  (bind _mindist (Variables|Default|GetMinDist))
  (bind _returnvalue (Math|Random|RandomFloatinRangefromStream _stream _maxdist _mindist))
  (Math|Random|SetRandomStreamSeed (LocalVariables|GetStream) (Variables|Default|Getseed))
  (Spline|ClearSplinePoints (Variables|Default|GetSpline) true)
  (Spline|AddSplinePoint (Variables|Default|GetSpline) (LocalVariables|GetCurrentLoc) "Local" true)
  (for _index (range 1 (- (Variables|Default|GetNBpoints) 1))
    (Spline|AddSplinePoint (Variables|Default|GetSpline) (+ (* (Math|Vector|MakeVector _returnvalue _returnvalue _returnvalue) (Class|KismetMathLibrary|VectorNormalUnsafe (Math|Vector|RotateVector (LocalVariables|GetCurrentDir) (Math|Rotator|MakeRotator (Math|Random|RandomFloatinRangefromStream (LocalVariables|GetStream) (- 0.0 (Variables|Default|GetJitter)) (Variables|Default|GetJitter)) (Math|Random|RandomFloatinRangefromStream (LocalVariables|GetStream) (- 0.0 (Variables|Default|GetJitter)) (Variables|Default|GetJitter)) 0.0)))) (LocalVariables|GetCurrentLoc)) "Local" true)
    (LocalVariables|SetCurrentLoc (+ (* (Math|Vector|MakeVector _returnvalue _returnvalue _returnvalue) (Class|KismetMathLibrary|VectorNormalUnsafe (Math|Vector|RotateVector (LocalVariables|GetCurrentDir) (Math|Rotator|MakeRotator (Math|Random|RandomFloatinRangefromStream (LocalVariables|GetStream) (- 0.0 (Variables|Default|GetJitter)) (Variables|Default|GetJitter)) (Math|Random|RandomFloatinRangefromStream (LocalVariables|GetStream) (- 0.0 (Variables|Default|GetJitter)) (Variables|Default|GetJitter)) 0.0)))) (LocalVariables|GetCurrentLoc)))
    (LocalVariables|SetCurrentDir (+ (* (Math|Vector|MakeVector _returnvalue _returnvalue _returnvalue) (Class|KismetMathLibrary|VectorNormalUnsafe (Math|Vector|RotateVector (LocalVariables|GetCurrentDir) (Math|Rotator|MakeRotator (Math|Random|RandomFloatinRangefromStream (LocalVariables|GetStream) (- 0.0 (Variables|Default|GetJitter)) (Variables|Default|GetJitter)) (Math|Random|RandomFloatinRangefromStream (LocalVariables|GetStream) (- 0.0 (Variables|Default|GetJitter)) (Variables|Default|GetJitter)) 0.0)))) (LocalVariables|GetCurrentLoc)))))