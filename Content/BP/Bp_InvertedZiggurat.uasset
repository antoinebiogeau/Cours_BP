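; Construction-script Blueprint that builds an inverted stepped ziggurat from instances of a stone mesh.
; It assigns the mesh to the Cube instanced component and uses its local bounds height to stack StoneZ layers upward from an offset.
; Each layer's X and Y scale grows with its index, so the tower widens toward the top.
; Three custom data floats are reserved but never written, and the event graph is empty.
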(event EventBeginPlay)

(event Collision|EventActorBeginOverlap
  (params (OtherActor :type Actor%20Object%20Reference)))

(event EventTick
  (params (DeltaSeconds :type Float%20%28single-precision%29)))

(fn ConstructionScript
  (bind _cube (Variables|Default|Getcube))
  (bind (_min _max) (Components|StaticMesh|GetLocalBounds _cube))
  (Class|InstancedStaticMeshComponent|SetNumCustomDataFloats (Variables|Default|Getcube) 3)
  ;[1 1 1] set static mesh et material
  (Components|StaticMesh|SetStaticMesh (Variables|Default|Getcube) (Variables|Default|GetSM_Stone))
  (LocalVariables|Setcenter (- _max _min))
  (for _index (range 0 (- (Variables|Default|GetStone%20Z) 1))
    (bind _output_get (LocalVariables|Seti _index))
    (bind _output_get_2 (LocalVariables|Setloc (Math|Vector|MakeVector 0.0 0.0 (+ (* _output_get (.z (LocalVariables|Getcenter))) (Variables|Default|GetOffset)))))
    (Components|InstancedStaticMesh|AddInstance (Variables|Default|Getcube) (Math|Transform|MakeTransform _output_get_2 "0, 0, 0" (Math|Vector|MakeVector (Math|Conversions|ToFloat(Integer) (+ _output_get 1)) (Math|Conversions|ToFloat(Integer) (+ _output_get 1)) 1.0)) false)))