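; Construction-script Blueprint that builds a vertical X-by-Y wall of mesh instances, with a random color for each column along X.
; It sets the mesh and material on the Cube instanced component, then spaces instances edge to edge using the mesh's local bounds.
; Each column's RGB is written to three per-instance custom data floats, presumably read by the material.
; RandX and RandY are computed but never used.
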(fn ConstructionScript
  (bind _cube (Variables|Default|Getcube))
  (bind _cube_2 (Variables|Default|Getcube))
  (bind (_min _max) (Components|StaticMesh|GetLocalBounds _cube_2))
  (LocalVariables|SetRandX (Math|Random|RandomIntegerinRange 0 (- (Variables|Default|GetX) 1)))
  (LocalVariables|SetRandY (Math|Random|RandomIntegerinRange 0 (- (Variables|Default|GetY) 1)))
  (Class|InstancedStaticMeshComponent|SetNumCustomDataFloats (Variables|Default|Getcube) 3)
  ;[1 1 1] set static mesh et material
  (Components|StaticMesh|SetStaticMesh _cube (Variables|Default|GetSM_Stone))
  (Rendering|Material|SetMaterial _cube 0 (Variables|Default|GetMaterial))
  (LocalVariables|Setcenter (- _max _min))
  (for _index (range 0 (- (Variables|Default|GetX) 1))
    (LocalVariables|Seti _index)
    (LocalVariables|Setlinear%20color (Utilities|Struct|MakeLinearColor (Math|Random|RandomFloat) (Math|Random|RandomFloat) (Math|Random|RandomFloat) 1.0))
    (for _index_2 (range 0 (- (Variables|Default|GetY) 1))
      (LocalVariables|Setj _index_2)
      (bind _returnvalue (Components|InstancedStaticMesh|AddInstance (Variables|Default|Getcube) (Math|Transform|MakeTransform (Math|Vector|MakeVector (* (.x (LocalVariables|Getcenter)) (LocalVariables|Geti)) 0.0 (+ (* (.z (LocalVariables|Getcenter)) (LocalVariables|Getj)) 5e+01)) "0, 0, 0" "1.000000,1.000000,1.000000") false))
      ;[1 1 1] custom data
      (Components|InstancedStaticMesh|SetCustomDataValue (Variables|Default|Getcube) _returnvalue 0 (.r (LocalVariables|Getlinear%20color)) false)
      (Components|InstancedStaticMesh|SetCustomDataValue (Variables|Default|Getcube) _returnvalue 1 (.g (LocalVariables|Getlinear%20color)) false)
      (Components|InstancedStaticMesh|SetCustomDataValue (Variables|Default|Getcube) _returnvalue 2 (.b (LocalVariables|Getlinear%20color)) false))))