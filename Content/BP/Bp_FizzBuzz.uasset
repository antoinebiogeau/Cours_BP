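; Actor that builds a vertical stack of stone mesh instances colored by FizzBuzz rules.
; The construction script adds StonesZ instances to an instanced mesh component, spaced by the mesh's bounds height plus a base Offset.
; Each one-based index is tested against FizzNum and BuzzNum to pick a Fizz, Buzz, FizzBuzz or other color.
; That color is written as RGB per-instance custom data alongside the assigned Material.
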(event EventBeginPlay)

(event Collision|EventActorBeginOverlap
  (params (OtherActor :type Actor%20Object%20Reference)))

(event EventTick
  (params (DeltaSeconds :type Float%20%28single-precision%29)))

(fn ConstructionScript
  (bind _cube (Variables|Default|Getcube))
  (bind _color_fizz_buzz (Variables|Default|GetColor%20Fizz%20Buzz))
  (bind _cube_2 (Variables|Default|Getcube))
  (bind _cube_3 (Variables|Default|Getcube))
  (bind _color_fizz (Variables|Default|GetColor%20Fizz))
  (bind _colorbuzz (Variables|Default|GetColorBuzz))
  (bind _cube_4 (Variables|Default|Getcube))
  (bind _color_other (Variables|Default|GetColor%20Other))
  (bind _cube_5 (Variables|Default|Getcube))
  (bind (_min _max) (Components|StaticMesh|GetLocalBounds _cube_5))
  (bind (_r _g _b) (Math|Color|BreakColor _color_other))
  (bind (_r_2 _g_2 _b_2) (Math|Color|BreakColor _color_fizz_buzz))
  (bind (_r_3 _g_3 _b_3) (Math|Color|BreakColor _color_fizz))
  (bind (_r_4 _g_4 _b_4) (Math|Color|BreakColor _colorbuzz))
  (Class|InstancedStaticMeshComponent|SetNumCustomDataFloats (Variables|Default|Getcube) 3)
  ;[1 1 1] set static mesh et material
  (Components|StaticMesh|SetStaticMesh (Variables|Default|Getcube) (Variables|Default|GetSM_Stone))
  (Rendering|Material|SetMaterial (Variables|Default|Getcube) 0 (Variables|Default|GetMaterial))
  (LocalVariables|Setcenter (- _max _min))
  (for _index (range 0 (- (Variables|Default|GetStones%20Z) 1))
    (LocalVariables|Seti _index)
    (bind _returnvalue (Components|InstancedStaticMesh|AddInstance (Variables|Default|Getcube) (Math|Transform|MakeTransform (Math|Vector|MakeVector 0.0 0.0 (+ (* (.z (LocalVariables|Getcenter)) (LocalVariables|Geti)) (Variables|Default|GetOffset))) "0, 0, 0" "1.000000,1.000000,1.000000") false))
    (if (and (== (Math|Integer|%(Integer) (+ (LocalVariables|Geti) 1) (Variables|Default|GetFizzNum)) 0) (== (Math|Integer|%(Integer) (+ (LocalVariables|Geti) 1) (Variables|Default|GetBuzzNum)) 0))
      ;[1 1 1] both
      (Components|InstancedStaticMesh|SetCustomDataValue _cube _returnvalue 0 _r_2 false)
      (Components|InstancedStaticMesh|SetCustomDataValue _cube _returnvalue 1 _g_2 false)
      (Components|InstancedStaticMesh|SetCustomDataValue _cube _returnvalue 2 _b_2 false)
      (elif (== (Math|Integer|%(Integer) (+ (LocalVariables|Geti) 1) (Variables|Default|GetFizzNum)) 0)
        ;[1 1 1] fizz
        (Components|InstancedStaticMesh|SetCustomDataValue _cube_3 _returnvalue 0 _r_3 false)
        (Components|InstancedStaticMesh|SetCustomDataValue _cube_3 _returnvalue 1 _g_3 false)
        (Components|InstancedStaticMesh|SetCustomDataValue _cube_3 _returnvalue 2 _b_3 false)
        (elif (== (Math|Integer|%(Integer) (+ (LocalVariables|Geti) 1) (Variables|Default|GetBuzzNum)) 0)
          ;[1 1 1] buzz
          (Components|InstancedStaticMesh|SetCustomDataValue _cube_4 _returnvalue 0 _r_4 false)
          (Components|InstancedStaticMesh|SetCustomDataValue _cube_4 _returnvalue 1 _g_4 false)
          (Components|InstancedStaticMesh|SetCustomDataValue _cube_4 _returnvalue 2 _b_4 false)
          (else
            ;[1 1 1] other
            (Components|InstancedStaticMesh|SetCustomDataValue _cube_2 _returnvalue 0 _r false)
            (Components|InstancedStaticMesh|SetCustomDataValue _cube_2 _returnvalue 1 _g false)
            (Components|InstancedStaticMesh|SetCustomDataValue _cube_2 _returnvalue 2 _b false)))))))