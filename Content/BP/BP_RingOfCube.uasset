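; BP_RingOfCube is a procedural placement actor that builds a ring of stone mesh instances in its Construction Script, with no runtime logic.
; It spaces CubeNum instances at equal angles on a circle of the given Radius, raised by half the mesh's height taken from its local bounds.
; Each instance faces radially outward, and the Rotation variable rotates both positions and orientations to tilt the whole ring.
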(event EventBeginPlay)

(event Collision|EventActorBeginOverlap
  (params (OtherActor :type Actor%20Object%20Reference)))

(event EventTick
  (params (DeltaSeconds :type Float%20%28single-precision%29)))

(fn ConstructionScript
  (bind _rotation (Variables|Default|GetRotation))
  (bind _cube (Variables|Default|Getcube))
  (bind (_min _max) (Components|StaticMesh|GetLocalBounds _cube))
  ;[1 1 1] set static mesh et material
  (Components|StaticMesh|SetStaticMesh (Variables|Default|Getcube) (Variables|Default|GetSM_Stone))
  (bind _output_get (LocalVariables|Setcenter (- _max _min)))
  (LocalVariables|SetHalfHeight%20 (/ (.z _output_get) 2.0))
  (LocalVariables|SetStepAngle%20 (/ 3.6e+02 (Math|Conversions|ToFloat(Integer) (Variables|Default|GetCube%20num))))
  (for _index (range 0 (- (Variables|Default|GetCube%20num) 1))
    (LocalVariables|Setindex _index)
    (bind _output_get_2 (LocalVariables|SetAngleDeg%20 (* (LocalVariables|Getindex) (LocalVariables|GetStepAngle%20))))
    (LocalVariables|SetAngleRad%20 (Math|Trig|DegreesToRadians _output_get_2))
    (LocalVariables|SetDri (Math|Vector|MakeVector (Math|Trig|Cos(Radians) (LocalVariables|GetAngleRad%20)) (Math|Trig|Sin(Radians) (LocalVariables|GetAngleRad%20)) 0.0))
    (bind _output_get_3 (LocalVariables|SetLocRel%20 (Math|Vector|MakeVector (* (.x (LocalVariables|GetDri)) (Variables|Default|GetRadius)) (* (.y (LocalVariables|GetDri)) (Variables|Default|GetRadius)) (LocalVariables|GetHalfHeight%20))))
    (bind _output_get_4 (LocalVariables|SetLowWorld (Math|Vector|RotateVector _output_get_3 _rotation)))
    (LocalVariables|SetRotInst%20 (Math|Rotator|CombineRotators (Math|Rotator|MakeRotfromX (LocalVariables|GetDri)) _rotation))
    (Components|InstancedStaticMesh|AddInstance (Variables|Default|Getcube) (Math|Transform|MakeTransform _output_get_4 (Math|Rotator|CombineRotators (Math|Rotator|MakeRotfromX (LocalVariables|GetDri)) _rotation) "1.000000,1.000000,1.000000") false)))