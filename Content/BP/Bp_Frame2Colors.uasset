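; Bp_Frame2Colors is an actor that builds a two-color framed wall of stone meshes in its Construction Script.
; It fills an X by Z grid of instances on an instanced static mesh component, spaced by the mesh's bounds with a vertical offset.
; Border instances get ColorA and inner ones ColorB, written as RGB into per-instance custom data for the assigned material.
; The event graph holds no active logic.
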(event EventBeginPlay)

(event Collision|EventActorBeginOverlap
  (params (OtherActor :type Actor%20Object%20Reference)))

(event EventTick
  (params (DeltaSeconds :type Float%20%28single-precision%29)))

(fn ConstructionScript
  (bind _color_a (Variables|Default|GetColor%20A))
  (bind _cube (Variables|Default|Getcube))
  (bind _color_b (Variables|Default|GetColor%20B))
  (bind (_r _g _b) (Math|Color|BreakColor _color_a))
  (bind (_r_2 _g_2 _b_2) (Math|Color|BreakColor _color_b))
  (bind (_min _max) (Components|StaticMesh|GetLocalBounds _cube))
  (Class|InstancedStaticMeshComponent|SetNumCustomDataFloats (Variables|Default|Getcube) 3)
  ;[1 1 1] set static mesh et material
  (Components|StaticMesh|SetStaticMesh (Variables|Default|Getcube) (Variables|Default|GetSM_Stone))
  (Rendering|Material|SetMaterial (Variables|Default|Getcube) 0 (Variables|Default|GetMaterial))
  (LocalVariables|Setcenter (- _max _min))
  (for _index (range 0 (- (Variables|Default|GetStone%20X) 1))
    (LocalVariables|Seti _index)
    (for _index_2 (range 0 (- (Variables|Default|GetStone%20Z) 1))
      (LocalVariables|Setj _index_2)
      (bind _returnvalue (Components|InstancedStaticMesh|AddInstance (Variables|Default|Getcube) (Math|Transform|MakeTransform (Math|Vector|MakeVector (* (.x (LocalVariables|Getcenter)) (LocalVariables|Geti)) 0.0 (+ (* (.z (LocalVariables|Getcenter)) (LocalVariables|Getj)) (Variables|Default|GetOffset))) "0, 0, 0" "1.000000,1.000000,1.000000") false))
      (LocalVariables|Setindex%20instance _returnvalue)
      (if (Math|Boolean|ORBoolean (or (== (LocalVariables|Geti) 0) (== (LocalVariables|Geti) (- (Variables|Default|GetStone%20X) 1))) (or (== (LocalVariables|Getj) 0) (== (LocalVariables|Getj) (- (Variables|Default|GetStone%20Z) 1))) (and (or (== (LocalVariables|Geti) 0) (== (LocalVariables|Geti) (- (Variables|Default|GetStone%20X) 1))) (or (== (LocalVariables|Getj) 0) (== (LocalVariables|Getj) (- (Variables|Default|GetStone%20Z) 1)))))
        (Components|InstancedStaticMesh|SetCustomDataValue (Variables|Default|Getcube) (LocalVariables|Getindex%20instance) 0 _r false)
        (Components|InstancedStaticMesh|SetCustomDataValue (Variables|Default|Getcube) (LocalVariables|Getindex%20instance) 1 _g false)
        (Components|InstancedStaticMesh|SetCustomDataValue (Variables|Default|Getcube) (LocalVariables|Getindex%20instance) 2 _b false)
        (else
          (Components|InstancedStaticMesh|SetCustomDataValue (Variables|Default|Getcube) (LocalVariables|Getindex%20instance) 0 _r_2 false)
          (Components|InstancedStaticMesh|SetCustomDataValue (Variables|Default|Getcube) (LocalVariables|Getindex%20instance) 1 _g_2 false)
          (Components|InstancedStaticMesh|SetCustomDataValue (Variables|Default|Getcube) (LocalVariables|Getindex%20instance) 2 _b_2 false))))))