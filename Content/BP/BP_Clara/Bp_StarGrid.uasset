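; Bp_StarGrid is a construction-script actor that builds a vertical XZ grid of instanced rock meshes from row, column and offset parameters.
; Nested loops space instances by mesh bounds plus offset, while a text render shows the class name and rock count.
; Three per-instance custom data floats give every third diagonal different values from the rest, likely as material colors.
; An invalid mesh or too-small grid prints an error.
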(event EventBeginPlay)

(event Collision|EventActorBeginOverlap
  (params (OtherActor :type Actor%20Object%20Reference)))

(event EventTick
  (params (DeltaSeconds :type Float%20%28single-precision%29)))

(fn ConstructionScript
  (bind _ism (Variables|Default|GetISM))
  (bind _ism_2 (Variables|Default|GetISM))
  (bind _offset (Variables|Default|GetOffset))
  (bind _ism_3 (Variables|Default|GetISM))
  (bind _ism_4 (Variables|Default|GetISM))
  (bind (_min _max) (Components|StaticMesh|GetLocalBounds _ism_2))
  ;[0.15 0.15 0.15 0.5] Setup
  (Class|InstancedStaticMeshComponent|SetNumCustomDataFloats (Variables|Default|GetISM) 3)
  (if (Utilities|IsValid (Variables|Default|GetSM%20Rock))
    (Components|InstancedStaticMesh|ClearInstances _ism)
    (Components|StaticMesh|SetStaticMesh _ism (Variables|Default|GetSM%20Rock))
    (if (and (> (Variables|Default|GetCols) 1) (> (Variables|Default|GetRows) 1))
      (Rendering|SetVisibility (Variables|Default|GetTextRender) true false)
      (Rendering|Material|SetMaterial (Variables|Default|GetISM) 0 (Variables|Default|GetMaterial))
      (Variables|Default|Setcenter (- _max _min))
      ;[0.15 0.15 0.15 0.5] Boucle XY
      (for _index (range 0 (- (Variables|Default|GetRows) 1))
        (LocalVariables|Seti _index)
        (for _index_2 (range 0 (- (Variables|Default|GetCols) 1))
          (LocalVariables|Setj _index_2)
          (bind _returnvalue (Components|InstancedStaticMesh|AddInstance (Variables|Default|GetISM) (Math|Transform|MakeTransform (Math|Vector|MakeVector (* (+ (.x (Variables|Default|Getcenter)) _offset) (LocalVariables|Geti)) 0.0 (+ (* (+ (.z (Variables|Default|Getcenter)) _offset) (LocalVariables|Getj)) _offset)) "0, 0, 0" "1.000000,1.000000,1.000000") false))
          (LocalVariables|SetInstance%20Index _returnvalue)
          (Rendering|Components|TextRender|SetText (Variables|Default|GetTextRender) (Utilities|Text|ToText(String) (Utilities|String|Append (Utilities|GetClassDisplayName "Bp_StarGrid_C") "  Rock Count: " (Utilities|String|ToString(Integer) (Components|InstancedStaticMesh|GetInstanceCount (Variables|Default|GetISM))))))
          (if (== (Math|Integer|%(Integer) (- (LocalVariables|Geti) (LocalVariables|Getj)) 3) 0)
            ;[0.15 0.15 0.15 0.5] Set materials
            (Components|InstancedStaticMesh|SetCustomDataValue _ism_4 (LocalVariables|GetInstance%20Index) 0 0.0 false)
            (Components|InstancedStaticMesh|SetCustomDataValue _ism_4 (LocalVariables|GetInstance%20Index) 1 0.0 false)
            (Components|InstancedStaticMesh|SetCustomDataValue _ism_4 (LocalVariables|GetInstance%20Index) 2 1.0 false)
            (else
              (Components|InstancedStaticMesh|SetCustomDataValue _ism_3 (LocalVariables|GetInstance%20Index) 0 0.0 false)
              (Components|InstancedStaticMesh|SetCustomDataValue _ism_3 (LocalVariables|GetInstance%20Index) 1 1.0 false)
              (Components|InstancedStaticMesh|SetCustomDataValue _ism_3 (LocalVariables|GetInstance%20Index) 2 0.0 false)))))
      (else
        (Development|PrintString "Erreur Param")
        (Rendering|SetVisibility (Variables|Default|GetTextRender) false false)))
    (else
      (Development|PrintString "MEsh invalide"))))