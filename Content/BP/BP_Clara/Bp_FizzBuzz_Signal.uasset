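; FizzBuzz signal Blueprint that builds a vertical stack of rock mesh instances colored by FizzBuzz rules.
; The Construction Script rebuilds the InstancedStaticMesh, spacing instances by mesh height plus an offset, and leaves the event graph unused.
; Each one-based index is tested against two divisors, and the matching color is written as per-instance custom data RGB.
; Invalid inputs print an error, and the rock count toggles TextRender visibility.
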(event EventBeginPlay)

(event Collision|EventActorBeginOverlap
  (params (OtherActor :type Actor%20Object%20Reference)))

(event EventTick
  (params (DeltaSeconds :type Float%20%28single-precision%29)))

(fn ConstructionScript
  (bind _ism (Variables|Default|GetISM))
  (bind _ism_2 (Variables|Default|GetISM))
  (bind _color_a___b (Variables|Default|GetColor%20A%20&%20B))
  (bind _color_a (Variables|Default|GetColor%20A))
  (bind _color_b (Variables|Default|GetColor%20B))
  (bind _color_other (Variables|Default|GetColor%20Other))
  (bind _ism_3 (Variables|Default|GetISM))
  (bind _ism_4 (Variables|Default|GetISM))
  (bind _ism_5 (Variables|Default|GetISM))
  (bind _ism_6 (Variables|Default|GetISM))
  (bind (_min _max) (Components|StaticMesh|GetLocalBounds _ism_2))
  (bind (_r _g _b) (Math|Color|BreakColor _color_other))
  (bind (_r_2 _g_2 _b_2) (Math|Color|BreakColor _color_a___b))
  (bind (_r_3 _g_3 _b_3) (Math|Color|BreakColor _color_a))
  (bind (_r_4 _g_4 _b_4) (Math|Color|BreakColor _color_b))
  ;[0.15 0.15 0.15 0.5] Setup
  (Class|InstancedStaticMeshComponent|SetNumCustomDataFloats (Variables|Default|GetISM) 3)
  (if (and (Utilities|IsValid (Variables|Default|GetSM%20Rock)) (Utilities|IsValid (Variables|Default|GetMaterial)))
    (Components|InstancedStaticMesh|ClearInstances _ism)
    (Components|StaticMesh|SetStaticMesh _ism (Variables|Default|GetSM%20Rock))
    (if (> (Variables|Default|GetRocks%20Z) 1)
      (Rendering|SetVisibility (Variables|Default|GetTextRender) true false)
      (Rendering|Material|SetMaterial (Variables|Default|GetISM) 0 (Variables|Default|GetMaterial))
      (bind _output_get (LocalVariables|Setcenter (- _max _min)))
      (for _index (range 0 (- (Variables|Default|GetRocks%20Z) 1))
        (LocalVariables|Seti _index)
        (bind _returnvalue (Components|InstancedStaticMesh|AddInstance (Variables|Default|GetISM) (Math|Transform|MakeTransform (Math|Vector|MakeVector 0.0 0.0 (+ (* (+ (.z _output_get) (Variables|Default|GetOffset)) (LocalVariables|Geti)) (Variables|Default|GetOffset))) "0, 0, 0" "1.000000,1.000000,1.000000") false))
        (if (and (== (Math|Integer|%(Integer) (+ (LocalVariables|Geti) 1) (Variables|Default|GetSignal%20A)) 0) (== (Math|Integer|%(Integer) (+ (LocalVariables|Geti) 1) (Variables|Default|GetSignal%20B)) 0))
          ;[1 1 1] both
          (Components|InstancedStaticMesh|SetCustomDataValue _ism_4 _returnvalue 0 _r_2 false)
          (Components|InstancedStaticMesh|SetCustomDataValue _ism_4 _returnvalue 1 _g_2 false)
          (Components|InstancedStaticMesh|SetCustomDataValue _ism_4 _returnvalue 2 _b_2 false)
          (elif (== (Math|Integer|%(Integer) (+ (LocalVariables|Geti) 1) (Variables|Default|GetSignal%20A)) 0)
            ;[1 1 1] fizz
            (Components|InstancedStaticMesh|SetCustomDataValue _ism_3 _returnvalue 0 _r_3 false)
            (Components|InstancedStaticMesh|SetCustomDataValue _ism_3 _returnvalue 1 _g_3 false)
            (Components|InstancedStaticMesh|SetCustomDataValue _ism_3 _returnvalue 2 _b_3 false)
            (elif (== (Math|Integer|%(Integer) (+ (LocalVariables|Geti) 1) (Variables|Default|GetSignal%20B)) 0)
              ;[1 1 1] buzz
              (Components|InstancedStaticMesh|SetCustomDataValue _ism_5 _returnvalue 0 _r_4 false)
              (Components|InstancedStaticMesh|SetCustomDataValue _ism_5 _returnvalue 1 _g_4 false)
              (Components|InstancedStaticMesh|SetCustomDataValue _ism_5 _returnvalue 2 _b_4 false)
              (else
                ;[1 1 1] other
                (Components|InstancedStaticMesh|SetCustomDataValue _ism_6 _returnvalue 0 _r false)
                (Components|InstancedStaticMesh|SetCustomDataValue _ism_6 _returnvalue 1 _g false)
                (Components|InstancedStaticMesh|SetCustomDataValue _ism_6 _returnvalue 2 _b false))))))
      (else
        (Development|PrintString "Erreur Param")
        (Rendering|SetVisibility (Variables|Default|GetTextRender) false false)))
    (else
      (Development|PrintString "MEsh invalide"))))