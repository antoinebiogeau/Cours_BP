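; BP_CometTower is an editor-configurable tower of stacked rock meshes, built entirely in the Construction Script with no runtime logic.
; It rebuilds an Instanced Static Mesh from SMRock, spacing RocksNUM-driven instances vertically by mesh height plus Offset, with evenly stepped rotation.
; A TextRender labels the class name and instance count.
; An invalid mesh or a count of one or less prints an error.
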(event EventBeginPlay)

(event Collision|EventActorBeginOverlap
  (params (OtherActor :type Actor%20Object%20Reference)))

(event EventTick
  (params (DeltaSeconds :type Float%20%28single-precision%29)))

(fn ConstructionScript
  (bind _ism (Variables|Default|GetISM))
  (bind _ism_2 (Variables|Default|GetISM))
  (bind (_min _max) (Components|StaticMesh|GetLocalBounds _ism_2))
  ;[0.15 0.15 0.15 0.5] Setup
  (Class|InstancedStaticMeshComponent|SetNumCustomDataFloats (Variables|Default|GetISM) 3)
  (if (Utilities|IsValid (Variables|Default|GetSM%20Rock))
    (Components|InstancedStaticMesh|ClearInstances _ism)
    (Components|StaticMesh|SetStaticMesh _ism (Variables|Default|GetSM%20Rock))
    (if (> (Variables|Default|GetRocks%20NUM) 1)
      (Rendering|SetVisibility (Variables|Default|GetTextRender) true false)
      (LocalVariables|Setcenter (- _max _min))
      (LocalVariables|Setangle%20step (/ 3.6e+02 (Math|Conversions|ToFloat(Integer) (- (Variables|Default|GetRocks%20NUM) 1))))
      (for _index (range 0 (- (Variables|Default|GetRocks%20NUM) 1))
        (bind _output_get (LocalVariables|Seti _index))
        (LocalVariables|Setangle (* (Math|Conversions|ToFloat(Integer) _output_get) (LocalVariables|Getangle%20step)))
        (LocalVariables|SetPos (Math|Vector|MakeVector 0.0 0.0 (+ (* (+ (.z (LocalVariables|Getcenter)) (Variables|Default|Getoffset)) (LocalVariables|Geti)) 5e+01)))
        (LocalVariables|SetRot (Math|Rotator|MakeRotator 0.0 0.0 (LocalVariables|Getangle)))
        (Components|InstancedStaticMesh|AddInstance (Variables|Default|GetISM) (Math|Transform|MakeTransform (LocalVariables|GetPos) (LocalVariables|GetRot)) false)
        (Rendering|Components|TextRender|SetText (Variables|Default|GetTextRender) (Utilities|Text|ToText(String) (Utilities|String|Append (Utilities|GetClassDisplayName "BP_CometTower_C") "  Rock Count: " (Utilities|String|ToString(Integer) (Components|InstancedStaticMesh|GetInstanceCount (Variables|Default|GetISM)))))))
      (else
        (Development|PrintString "Erreur Param")
        (Rendering|SetVisibility (Variables|Default|GetTextRender) false false)))
    (else
      (Development|PrintString "MEsh invalide"))))