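; Construction-script tool that lays out rock meshes along a flat spiral as instances of one instanced static mesh.
; Each rock's angle, radius and scale grow with its index from turn count and max radius, and a shared rotation tilts the whole spiral.
; Three random custom data floats per instance supply color variation to the material.
; A text label shows the class name and rock count, and invalid inputs print errors.
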(event EventBeginPlay)

(event Collision|EventActorBeginOverlap
  (params (OtherActor :type Actor%20Object%20Reference)))

(event EventTick
  (params (DeltaSeconds :type Float%20%28single-precision%29)))

(fn ConstructionScript
  (bind _returnvalue (Math|Random|RandomFloat))
  (bind _rotation (Variables|Default|GetRotation))
  (bind _ism (Variables|Default|GetISM))
  (bind _ism_2 (Variables|Default|GetISM))
  (bind (_min _max) (Components|StaticMesh|GetLocalBounds _ism_2))
  ;[0.15 0.15 0.15 0.5] Check et setup
  (Class|InstancedStaticMeshComponent|SetNumCustomDataFloats (Variables|Default|GetISM) 3)
  (if (and (Utilities|IsValid (Variables|Default|GetSM_Rock)) (Utilities|IsValid (Variables|Default|GetMaterial)))
    (Components|InstancedStaticMesh|ClearInstances (Variables|Default|GetISM))
    (if (> (Variables|Default|GetRocks%20NUM) 1)
      (Rendering|Material|SetMaterial (Variables|Default|GetISM) 0 (Variables|Default|GetMaterial))
      (Rendering|SetVisibility (Variables|Default|GetTextRender) true false)
      ;[1 1 1] set static mesh et material
      (Components|StaticMesh|SetStaticMesh (Variables|Default|GetISM) (Variables|Default|GetSM_Rock))
      (bind _output_get (LocalVariables|Setcenter (- _max _min)))
      (LocalVariables|SetHalfHeight%20 (/ (.z _output_get) 2.0))
      (LocalVariables|SetStepAngle%20 (/ 3.6e+02 (Math|Conversions|ToFloat(Integer) (Variables|Default|GetRocks%20NUM))))
      (for _index (range 0 (- (Variables|Default|GetRocks%20NUM) 1))
        (bind _output_get_2 (LocalVariables|Setindex _index))
        ;[0.15 0.15 0.15 0.5] Ratio T pour la spiral
        (bind _output_get_3 (LocalVariables|Sett (/ (Math|Conversions|ToFloat(Integer) _output_get_2) (Variables|Default|GetRocks%20NUM))))
        (bind _output_get_4 (LocalVariables|SetAngleDeg%20 (* (* _output_get_3 (Variables|Default|GetTurns)) 3.6e+02)))
        (LocalVariables|SetAngleRad%20 (Math|Trig|DegreesToRadians _output_get_4))
        (LocalVariables|SetRadius (* (LocalVariables|Gett) (Variables|Default|GetRadius%20Max%20)))
        (LocalVariables|SetScale (* (+ (LocalVariables|Gett) 0.2) 0.8))
        (bind _output_get_5 (LocalVariables|SetDri (Math|Vector|MakeVector (* (Math|Trig|Cos(Radians) (LocalVariables|GetAngleRad%20)) (LocalVariables|GetRadius)) (* (Math|Trig|Sin(Radians) (LocalVariables|GetAngleRad%20)) (LocalVariables|GetRadius)) 0.0)))
        (bind _output_get_6 (LocalVariables|SetLowWorld (Math|Vector|RotateVector _output_get_5 _rotation)))
        (bind _returnvalue_2 (Components|InstancedStaticMesh|AddInstance (Variables|Default|GetISM) (Math|Transform|MakeTransform _output_get_6 (Math|Rotator|CombineRotators (Math|Rotator|MakeRotfromX (LocalVariables|GetDri)) _rotation) (Math|Vector|MakeVector (LocalVariables|GetScale) (LocalVariables|GetScale) (LocalVariables|GetScale))) false))
        (LocalVariables|SetInstance%20Index _returnvalue_2)
        (Rendering|Components|TextRender|SetText (Variables|Default|GetTextRender) (Utilities|Text|ToText(String) (Utilities|String|Append (Utilities|GetClassDisplayName "Bp_OrbitChain_C") "  Rock Count: " (Utilities|String|ToString(Integer) (Components|InstancedStaticMesh|GetInstanceCount (Variables|Default|GetISM))))))
        ;[0.15 0.15 0.15 0.5] RND color
        (Components|InstancedStaticMesh|SetCustomDataValue _ism (LocalVariables|GetInstance%20Index) 0 _returnvalue false)
        (Components|InstancedStaticMesh|SetCustomDataValue _ism (LocalVariables|GetInstance%20Index) 1 _returnvalue false)
        (Components|InstancedStaticMesh|SetCustomDataValue _ism (LocalVariables|GetInstance%20Index) 2 _returnvalue false))
      (else
        (Development|PrintString "Erreur Param")
        (Rendering|SetVisibility (Variables|Default|GetTextRender) false false)))
    (else
      (Development|PrintString "MEsh invalide"))))