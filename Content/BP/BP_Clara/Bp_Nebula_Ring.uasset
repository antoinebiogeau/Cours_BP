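; Construction-script actor that lays out a ring of rock meshes as instanced static mesh instances.
; Spaces RocksNUM copies of SMRock evenly around Radius, facing outward, offset by half the ISM bounds height and turned by Rotation.
; A text render shows the class name and instance count; an invalid mesh or count prints an error.
; Reserves three custom data floats per instance but writes none; no runtime logic.
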(event EventBeginPlay)

(event Collision|EventActorBeginOverlap
  (params (OtherActor :type Actor%20Object%20Reference)))

(event EventTick
  (params (DeltaSeconds :type Float%20%28single-precision%29)))

(fn ConstructionScript
  (bind _rotation (Variables|Default|GetRotation))
  (bind _ism (Variables|Default|GetISM))
  (bind (_min _max) (Components|StaticMesh|GetLocalBounds _ism))
  ;[0.15 0.15 0.15 0.5] setup et check
  (Class|InstancedStaticMeshComponent|SetNumCustomDataFloats (Variables|Default|GetISM) 3)
  (if (Utilities|IsValid (Variables|Default|GetSM_Rock))
    (Components|InstancedStaticMesh|ClearInstances (Variables|Default|GetISM))
    (if (> (Variables|Default|GetRocks%20NUM) 1)
      (Rendering|SetVisibility (Variables|Default|GetTextRender) true false)
      ;[1 1 1] set static mesh et material
      (Components|StaticMesh|SetStaticMesh (Variables|Default|GetISM) (Variables|Default|GetSM_Rock))
      (bind _output_get (LocalVariables|Setcenter (- _max _min)))
      (LocalVariables|SetHalfHeight%20 (/ (.z _output_get) 2.0))
      (LocalVariables|SetStepAngle%20 (/ 3.6e+02 (Math|Conversions|ToFloat(Integer) (Variables|Default|GetRocks%20NUM))))
      (for _index (range 0 (- (Variables|Default|GetRocks%20NUM) 1))
        (LocalVariables|Setindex _index)
        (bind _output_get_2 (LocalVariables|SetAngleDeg%20 (* (LocalVariables|Getindex) (LocalVariables|GetStepAngle%20))))
        (LocalVariables|SetAngleRad%20 (Math|Trig|DegreesToRadians _output_get_2))
        (LocalVariables|SetDri (Math|Vector|MakeVector (Math|Trig|Cos(Radians) (LocalVariables|GetAngleRad%20)) (Math|Trig|Sin(Radians) (LocalVariables|GetAngleRad%20)) 0.0))
        (bind _output_get_3 (LocalVariables|SetLocRel%20 (Math|Vector|MakeVector (* (.x (LocalVariables|GetDri)) (Variables|Default|GetRadius)) (* (.y (LocalVariables|GetDri)) (Variables|Default|GetRadius)) (LocalVariables|GetHalfHeight%20))))
        (bind _output_get_4 (LocalVariables|SetLowWorld (Math|Vector|RotateVector _output_get_3 _rotation)))
        (LocalVariables|SetRotInst%20 (Math|Rotator|CombineRotators (Math|Rotator|MakeRotfromX (LocalVariables|GetDri)) _rotation))
        (bind _returnvalue (Components|InstancedStaticMesh|AddInstance (Variables|Default|GetISM) (Math|Transform|MakeTransform _output_get_4 (Math|Rotator|CombineRotators (Math|Rotator|MakeRotfromX (LocalVariables|GetDri)) _rotation)) false))
        (LocalVariables|SetInstance%20Index _returnvalue)
        (Rendering|Components|TextRender|SetText (Variables|Default|GetTextRender) (Utilities|Text|ToText(String) (Utilities|String|Append (Utilities|GetClassDisplayName "Bp_Nebula_Ring_C") "  Rock Count: " (Utilities|String|ToString(Integer) (Components|InstancedStaticMesh|GetInstanceCount (Variables|Default|GetISM)))))))
      (else
        (Development|PrintString "Erreur Param")
        (Rendering|SetVisibility (Variables|Default|GetTextRender) false false)))
    (else
      (Development|PrintString "MEsh invalide"))))