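; Procedural tree generator that builds trunk, branches, sub-branches and leaves in the construction script.
; A cone-constrained random walk lays the trunk spline; branch splines sprout along it and sub-branches along each branch.
; Spline mesh segments skin each spline with lerped radii, and branch points randomly receive scaled leaf instances.
; A seeded stream drives most randomness, but branch and sub-branch jitter uses unseeded cone vectors, so shapes are not fully reproducible.
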(event EventBeginPlay)

(event Collision|EventActorBeginOverlap
  (params (OtherActor :type Actor%20Object%20Reference)))

(event EventTick
  (params (DeltaSeconds :type Float%20%28single-precision%29)))

(fn ConstructionScript
  (bind _stream (LocalVariables|Getstream))
  (bind _stream_2 (LocalVariables|Getstream))
  (bind _stream_3 (LocalVariables|Getstream))
  (bind _returnvalue (Math|Random|RandomFloatinRangefromStream _stream 2.0 4.0))
  ;[1 1 1] spawn du trnc
  (Math|Random|SetRandomStreamSeed (LocalVariables|Getstream) (Variables|Default|GetNew%20Seed))
  (Spline|ClearSplinePoints (Variables|Default|GetSpline) true)
  (Spline|AddSplinePoint (Variables|Default|GetSpline) (LocalVariables|GetcurrentLoc) "Local" true)
  (for _index (range 1 (- (Variables|trunc|GetNBTruncPoint) 1))
    (LocalVariables|Seti _index)
    (LocalVariables|SetRandDist (Math|Random|RandomFloatinRangefromStream (LocalVariables|Getstream) (Variables|trunc|GetMinDistPointTrunc) (Variables|trunc|GetMaxDistPointTrunc)))
    (LocalVariables|SetRandDir (Math|Random|RandomUnitVectorinConeinDegreesfromStream (LocalVariables|Getstream) (LocalVariables|GetCurrentDir) (Variables|trunc|GetAngle)))
    (bind _output_get (LocalVariables|SetnextLoc (+ (LocalVariables|GetcurrentLoc) (* (LocalVariables|GetRandDist) (LocalVariables|GetRandDir)))))
    (Spline|AddSplinePoint (Variables|Default|GetSpline) _output_get "Local" true)
    (LocalVariables|SetcurrentLoc (LocalVariables|GetnextLoc))
    (LocalVariables|SetCurrentDir (LocalVariables|GetRandDir)))
  ;[1 1 1] habillage du tronc
  (for _index_2 (range 0 (- (Variables|trunc|GetNBTruncPoint) 2))
    (LocalVariables|Seti _index_2)
    (bind _returnvalue_2 (AddComponent|AddSplineMeshComponent false))
    (SplineMesh|SetStartandEnd _returnvalue_2 (.position (Spline|GetSplinePointAt (Variables|Default|GetSpline) (LocalVariables|Geti) "Local")) (.arrivetangent (Spline|GetSplinePointAt (Variables|Default|GetSpline) (LocalVariables|Geti) "Local")) (.position (Spline|GetSplinePointAt (Variables|Default|GetSpline) (+ (LocalVariables|Geti) 1) "Local")) (.leavetangent (Spline|GetSplinePointAt (Variables|Default|GetSpline) (+ (LocalVariables|Geti) 1) "Local")) true :!class /Script/Engine.SplineMeshComponent)
    (SplineMesh|SetStartScale _returnvalue_2 (Math|Vector2D|MakeVector2D (Math|Float|Lerp (Variables|trunc|GetBaseraduis) (Variables|trunc|GetToprad) (/ (Spline|GetDistanceAlongSplineatSplinePoint (Variables|Default|GetSpline) (LocalVariables|Geti)) (Spline|GetSplineLength (Variables|Default|GetSpline)))) (Math|Float|Lerp (Variables|trunc|GetBaseraduis) (Variables|trunc|GetToprad) (/ (Spline|GetDistanceAlongSplineatSplinePoint (Variables|Default|GetSpline) (LocalVariables|Geti)) (Spline|GetSplineLength (Variables|Default|GetSpline))))) true :!class /Script/Engine.SplineMeshComponent)
    (SplineMesh|SetEndScale _returnvalue_2 (Math|Vector2D|MakeVector2D (Math|Float|Lerp (Variables|trunc|GetBaseraduis) (Variables|trunc|GetToprad) (/ (Spline|GetDistanceAlongSplineatSplinePoint (Variables|Default|GetSpline) (+ (LocalVariables|Geti) 1)) (Spline|GetSplineLength (Variables|Default|GetSpline)))) (Math|Float|Lerp (Variables|trunc|GetBaseraduis) (Variables|trunc|GetToprad) (/ (Spline|GetDistanceAlongSplineatSplinePoint (Variables|Default|GetSpline) (+ (LocalVariables|Geti) 1)) (Spline|GetSplineLength (Variables|Default|GetSpline))))) true :!class /Script/Engine.SplineMeshComponent))
  ;[1 1 1] generation de branch
  (for _index_3 (range 0 (- (Variables|Branch|GetNbBranch) 1))
    (bind _output_get_2 (LocalVariables|SetRandRatio%20%20%20 (Math|Random|RandomFloatinRangefromStream (LocalVariables|Getstream) (Variables|Branch|GetBranchStart) 1.0)))
    (bind _output_get_3 (LocalVariables|SetSpawnDist (* _output_get_2 (Spline|GetSplineLength (Variables|Default|GetSpline)))))
    (bind _returnvalue_3 (AddComponent|AddSplineComponent false))
    (Spline|ClearSplinePoints _returnvalue_3 true)
    (LocalVariables|SetCurrentLocBranch (Spline|GetLocationatDistanceAlongSpline (Variables|Default|GetSpline) _output_get_3 "Local"))
    (bind _output_get_4 (LocalVariables|SetBranchtangeant (Spline|GetTangentatDistanceAlongSpline (Variables|Default|GetSpline) _output_get_3 "Local")))
    (bind _output_get_5 (LocalVariables|SetBaseDir (Math|Vector|RotateVectorAroundAxis _output_get_4 (Math|Random|RandomFloatinRangefromStream _stream_3 9e+01 -9e+01) (Math|Random|RandomUnitVectorfromStream _stream_3))))
    (LocalVariables|SetCurrentDirBranch _output_get_5)
    (for _index_4 (range 0 (- (Variables|Branch|GetNbPointBranch) 1))
      (Spline|AddSplinePoint _returnvalue_3 (LocalVariables|GetCurrentLocBranch) "Local" true)
      (bind _output_get_6 (LocalVariables|SetnextLoc (+ (LocalVariables|GetCurrentLocBranch) (* (Math|Random|RandomUnitVectorinConeinDegrees (LocalVariables|GetCurrentDirBranch) (Variables|Branch|GetBranchJitterAngle)) (Math|Random|RandomIntegerinRangefromStream (LocalVariables|Getstream) (Variables|Branch|GetMin_BranchLenght) (Variables|Branch|GetMax_BranchLenght))))))
      (LocalVariables|SetCurrentLocBranch _output_get_6)
      (LocalVariables|SetCurrentDirBranch (Math|Random|RandomUnitVectorinConeinDegrees (LocalVariables|GetCurrentDirBranch) (Variables|Branch|GetBranchJitterAngle))))
    ;[1 1 1] habimlage bracnh
    (for _index_5 (range 0 (- (Variables|Branch|GetNbPointBranch) 2))
      (LocalVariables|Seti _index_5)
      (bind _returnvalue_4 (AddComponent|AddSplineMeshComponent false))
      (SplineMesh|SetStartandEnd _returnvalue_4 (.position (Spline|GetSplinePointAt _returnvalue_3 (LocalVariables|Geti) "Local")) (.arrivetangent (Spline|GetSplinePointAt _returnvalue_3 (LocalVariables|Geti) "Local")) (.position (Spline|GetSplinePointAt _returnvalue_3 (+ (LocalVariables|Geti) 1) "Local")) (.leavetangent (Spline|GetSplinePointAt _returnvalue_3 (+ (LocalVariables|Geti) 1) "Local")) true :!class /Script/Engine.SplineMeshComponent)
      (if (Variables|leaf|GetLeafs?)
        (if (> (LocalVariables|Geti) 1)
          (if (== (Math|Random|RandomIntegerinRangefromStream (LocalVariables|Getstream) 0 (Variables|leaf|GetprobaLeaf)) 1)
            (Components|InstancedStaticMesh|AddInstance (Variables|Default|Getleafs) (Math|Transform|MakeTransform (.position (Spline|GetSplinePointAt _returnvalue_3 (LocalVariables|Geti) "Local")) "0, 0, 0" (Math|Vector|MakeVector _returnvalue _returnvalue _returnvalue)) false))))
      (SplineMesh|SetStartScale _returnvalue_4 (Math|Vector2D|MakeVector2D (Math|Float|Lerp (Variables|Branch|GetTopRadBranch) (Variables|Branch|GetbaseRadBranch) (/ (Spline|GetDistanceAlongSplineatSplinePoint _returnvalue_3 (LocalVariables|Geti)) (Spline|GetSplineLength _returnvalue_3))) (Math|Float|Lerp (Variables|Branch|GetTopRadBranch) (Variables|Branch|GetbaseRadBranch) (/ (Spline|GetDistanceAlongSplineatSplinePoint _returnvalue_3 (LocalVariables|Geti)) (Spline|GetSplineLength _returnvalue_3)))) true :!class /Script/Engine.SplineMeshComponent)
      (SplineMesh|SetEndScale _returnvalue_4 (Math|Vector2D|MakeVector2D (Math|Float|Lerp (Variables|Branch|GetTopRadBranch) (Variables|Branch|GetbaseRadBranch) (/ (Spline|GetDistanceAlongSplineatSplinePoint _returnvalue_3 (+ (LocalVariables|Geti) 1)) (Spline|GetSplineLength _returnvalue_3))) (Math|Float|Lerp (Variables|Branch|GetTopRadBranch) (Variables|Branch|GetbaseRadBranch) (/ (Spline|GetDistanceAlongSplineatSplinePoint _returnvalue_3 (+ (LocalVariables|Geti) 1)) (Spline|GetSplineLength _returnvalue_3)))) true :!class /Script/Engine.SplineMeshComponent))
    ;[1 1 1] generation de branch
    (for _index_6 (range 0 (- (Variables|SubBranch|GetNbSub) 1))
      (bind _output_get_7 (LocalVariables|SetRandRatio%20%20%20 (Math|Random|RandomFloatinRangefromStream (LocalVariables|Getstream) (Variables|Branch|GetBranchStart) 1.0)))
      (bind _output_get_8 (LocalVariables|SetSpawnDist (* _output_get_7 (Spline|GetSplineLength _returnvalue_3))))
      (bind _returnvalue_5 (AddComponent|AddSplineComponent false))
      (Spline|ClearSplinePoints _returnvalue_5 true)
      (LocalVariables|SetCurrentLocBranch (Spline|GetLocationatDistanceAlongSpline _returnvalue_3 _output_get_8 "Local"))
      (bind _output_get_9 (LocalVariables|SetBranchtangeant (Spline|GetTangentatDistanceAlongSpline _returnvalue_3 _output_get_8 "Local")))
      (bind _output_get_10 (LocalVariables|SetBaseDir (Math|Vector|RotateVectorAroundAxis _output_get_9 (Math|Random|RandomFloatinRangefromStream _stream_2 9e+01 -9e+01) (Math|Random|RandomUnitVectorfromStream _stream_2))))
      (LocalVariables|SetCurrentDirBranch _output_get_10)
      (for _index_7 (range 0 (- (Variables|SubBranch|GetNbPointSubBranch) 1))
        (Spline|AddSplinePoint _returnvalue_5 (LocalVariables|GetCurrentLocBranch) "Local" true)
        (bind _output_get_11 (LocalVariables|SetnextLoc (+ (LocalVariables|GetCurrentLocBranch) (* (Math|Random|RandomUnitVectorinConeinDegrees (LocalVariables|GetCurrentDirBranch) (Variables|Branch|GetBranchJitterAngle)) (Math|Random|RandomIntegerinRangefromStream (LocalVariables|Getstream) (Variables|SubBranch|GetMinSubLenght) (Variables|SubBranch|GetMaxSubLength))))))
        (LocalVariables|SetCurrentLocBranch _output_get_11)
        (LocalVariables|SetCurrentDirBranch (Math|Random|RandomUnitVectorinConeinDegrees (LocalVariables|GetCurrentDirBranch) (Variables|Branch|GetBranchJitterAngle))))
      ;[1 1 1] habimlage bracnh
      (for _index_8 (range 0 (- (Variables|SubBranch|GetNbPointSubBranch) 2))
        (LocalVariables|Seti _index_8)
        (bind _returnvalue_6 (AddComponent|AddSplineMeshComponent false))
        (SplineMesh|SetStartandEnd _returnvalue_6 (.position (Spline|GetSplinePointAt _returnvalue_5 (LocalVariables|Geti) "Local")) (.arrivetangent (Spline|GetSplinePointAt _returnvalue_5 (LocalVariables|Geti) "Local")) (.position (Spline|GetSplinePointAt _returnvalue_5 (+ (LocalVariables|Geti) 1) "Local")) (.leavetangent (Spline|GetSplinePointAt _returnvalue_5 (+ (LocalVariables|Geti) 1) "Local")) true :!class /Script/Engine.SplineMeshComponent)
        (SplineMesh|SetStartScale _returnvalue_6 (Math|Vector2D|MakeVector2D (Math|Float|Lerp (Variables|SubBranch|GetBaseSub) (Variables|SubBranch|GetTopSUb) (/ (Spline|GetDistanceAlongSplineatSplinePoint _returnvalue_5 (LocalVariables|Geti)) (Spline|GetSplineLength _returnvalue_5))) (Math|Float|Lerp (Variables|SubBranch|GetBaseSub) (Variables|SubBranch|GetTopSUb) (/ (Spline|GetDistanceAlongSplineatSplinePoint _returnvalue_5 (LocalVariables|Geti)) (Spline|GetSplineLength _returnvalue_5)))) true :!class /Script/Engine.SplineMeshComponent)
        (SplineMesh|SetEndScale _returnvalue_6 (Math|Vector2D|MakeVector2D (Math|Float|Lerp (Variables|SubBranch|GetBaseSub) (Variables|SubBranch|GetTopSUb) (/ (Spline|GetDistanceAlongSplineatSplinePoint _returnvalue_5 (+ (LocalVariables|Geti) 1)) (Spline|GetSplineLength _returnvalue_5))) (Math|Float|Lerp (Variables|SubBranch|GetBaseSub) (Variables|SubBranch|GetTopSUb) (/ (Spline|GetDistanceAlongSplineatSplinePoint _returnvalue_5 (+ (LocalVariables|Geti) 1)) (Spline|GetSplineLength _returnvalue_5)))) true :!class /Script/Engine.SplineMeshComponent)))))