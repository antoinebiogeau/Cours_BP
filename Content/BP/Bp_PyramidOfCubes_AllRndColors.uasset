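; Actor Blueprint that builds a stepped pyramid of instanced stone meshes, each with its own random color values.
; The Construction Script sets mesh and material, then sizes the grid from the mesh's local bounds.
; Nested loops stack StoneZ centered square layers, each one stone narrower per side, raised by Offset.
; Each instance gets three random 0–1 custom data floats, rerolled whenever construction runs.
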(event EventBeginPlay)

(event Collision|EventActorBeginOverlap
  (params (OtherActor :type Actor%20Object%20Reference)))

(event EventTick
  (params (DeltaSeconds :type Float%20%28single-precision%29)))

(fn ConstructionScript
  (bind _returnvalue (Math|Random|RandomFloatinRange 0.0 1.0))
  (bind _cube (Variables|Default|Getcube))
  (bind (_min _max) (Components|StaticMesh|GetLocalBounds _cube))
  (Class|InstancedStaticMeshComponent|SetNumCustomDataFloats (Variables|Default|Getcube) 3)
  ;[1 1 1] set static mesh et material
  (Components|StaticMesh|SetStaticMesh (Variables|Default|Getcube) (Variables|Default|GetSM_Stone))
  (Rendering|Material|SetMaterial (Variables|Default|Getcube) 0 (Variables|Default|GetMaterial))
  (LocalVariables|Setcenter (- _max _min))
  (for _index (range 0 (- (Variables|Default|GetStone%20Z) 1))
    (LocalVariables|Seti _index)
    (LocalVariables|SetOffsetX%20 (/ (* (Utilities|Operators|Subtract (Variables|Default|GetStone%20Z) (LocalVariables|Geti) 1) (.x (LocalVariables|Getcenter))) 2.0))
    (LocalVariables|SetOffsetY%20 (/ (* (Utilities|Operators|Subtract (Variables|Default|GetStone%20Z) (LocalVariables|Geti) 1) (.y (LocalVariables|Getcenter))) 2.0))
    (LocalVariables|SetLocZ%20%20%20%20 (+ (* (.z (LocalVariables|Getcenter)) (LocalVariables|Geti)) (Variables|Default|GetOffset)))
    (for _index_2 (range 0 (- (- (Variables|Default|GetStone%20Z) (LocalVariables|Geti)) 1))
      (LocalVariables|Setj _index_2)
      (for _index_3 (range 0 (- (- (Variables|Default|GetStone%20Z) (LocalVariables|Geti)) 1))
        (LocalVariables|SetY _index_3)
        (bind _output_get (LocalVariables|Setloc (Math|Vector|MakeVector (- (* (LocalVariables|Getj) (.x (LocalVariables|Getcenter))) (LocalVariables|GetOffsetX%20)) (- (* (LocalVariables|GetY) (.y (LocalVariables|Getcenter))) (LocalVariables|GetOffsetY%20)) (LocalVariables|GetLocZ%20%20%20%20))))
        (bind _returnvalue_2 (Components|InstancedStaticMesh|AddInstance (Variables|Default|Getcube) (Math|Transform|MakeTransform _output_get "0, 0, 0" "1.000000,1.000000,1.000000") false))
        ;[1 1 1] custom data
        (Components|InstancedStaticMesh|SetCustomDataValue (Variables|Default|Getcube) _returnvalue_2 0 _returnvalue false)
        (Components|InstancedStaticMesh|SetCustomDataValue (Variables|Default|Getcube) _returnvalue_2 1 _returnvalue false)
        (Components|InstancedStaticMesh|SetCustomDataValue (Variables|Default|Getcube) _returnvalue_2 2 _returnvalue false)))))