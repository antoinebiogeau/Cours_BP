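; Construction-script Blueprint that builds a stone wall along a spline from instances of a chosen mesh.
; A nested loop spreads StoneX instances evenly along the spline length, following its rotation, and stacks StoneZ rows at a fixed height step plus Offset.
; Two text renders near the first spline point show the stone count and a Value label.
; Mesh bounds are computed but do not affect spacing.
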(event EventBeginPlay)

(event Collision|EventActorBeginOverlap
  (params (OtherActor :type Actor%20Object%20Reference)))

(event EventTick
  (params (DeltaSeconds :type Float%20%28single-precision%29)))

(fn ConstructionScript
  (bind _textrender1 (Variables|Default|GetTextRender1))
  (bind _spline (Variables|Default|GetSpline))
  (bind _cube (Variables|Default|Getcube))
  (bind _textrender (Variables|Default|GetTextRender))
  (bind (_min _max) (Components|StaticMesh|GetLocalBounds _cube))
  (bind _returnvalue (Spline|GetTransformatSplinePoint _spline 0 "World" false))
  (bind _returnvalue_2 (Math|Rotator|CombineRotators (.rotation _returnvalue) "0.000000,90.000000,0.000000"))
  (Rendering|Components|TextRender|SetText _textrender (Utilities|Text|ToText(String) (Utilities|String|Append (LocalVariables|Gettext1) (Utilities|String|ToString(Integer) (* (Variables|Default|GetStoneX) (Variables|Default|GetStoneZ))))))
  (Transformation|SetWorldTransform _textrender (Math|Transform|MakeTransform (+ (.location _returnvalue) (Math|Vector|MakeVector 0.0 1e+02 1e+02)) _returnvalue_2 "1.000000,1.000000,1.000000") false false)
  (Rendering|Components|TextRender|SetText _textrender1 (Variables|Default|GetValue))
  (Transformation|SetWorldTransform _textrender1 (Math|Transform|MakeTransform (+ (.location _returnvalue) (Math|Vector|MakeVector 0.0 1e+02 5e+01)) _returnvalue_2 "1.000000,1.000000,1.000000") false false)
  (Components|StaticMesh|SetStaticMesh (Variables|Default|Getcube) (Variables|Default|GetSM_Stone))
  (LocalVariables|SetNewLocalVar (- _max _min))
  (for _index (range 0 (- (Variables|Default|GetStoneZ) 1))
    (LocalVariables|SetZ _index)
    (for _index_2 (range 0 (- (Variables|Default|GetStoneX) 1))
      (LocalVariables|SetX _index_2)
      (LocalVariables|SetLenght (Spline|GetSplineLength (Variables|Default|GetSpline)))
      (bind _output_get (LocalVariables|Settransform (Math|Transform|MakeTransform (Math|Vector|MakeVector (.x (Spline|GetLocationatDistanceAlongSpline (Variables|Default|GetSpline) (* (/ (LocalVariables|GetX) (Math|Conversions|ToFloat(Integer) (- (Variables|Default|GetStoneX) 1))) (LocalVariables|GetLenght)) "Local")) (.y (Spline|GetLocationatDistanceAlongSpline (Variables|Default|GetSpline) (* (/ (LocalVariables|GetX) (Math|Conversions|ToFloat(Integer) (- (Variables|Default|GetStoneX) 1))) (LocalVariables|GetLenght)) "Local")) (+ (.z (Spline|GetLocationatDistanceAlongSpline (Variables|Default|GetSpline) (* (/ (LocalVariables|GetX) (Math|Conversions|ToFloat(Integer) (- (Variables|Default|GetStoneX) 1))) (LocalVariables|GetLenght)) "Local")) (Math|Conversions|ToFloat(Integer) (+ (* (LocalVariables|GetZ) 100) (Variables|Default|GetOffset))))) (Spline|GetRotationatDistanceAlongSpline (Variables|Default|GetSpline) (* (/ (LocalVariables|GetX) (Math|Conversions|ToFloat(Integer) (- (Variables|Default|GetStoneX) 1))) (LocalVariables|GetLenght)) "Local"))))
      (Components|InstancedStaticMesh|AddInstance (Variables|Default|Getcube) _output_get false))))