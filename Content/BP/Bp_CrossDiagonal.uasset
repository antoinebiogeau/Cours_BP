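; Construction-script Blueprint that builds an X-shaped cross of stone meshes in the local XZ plane.
; It loops over a StonesXZ-sized square grid and adds an instance to the instanced Cube component only on the two diagonals.
; Spacing comes from the mesh bounds; the cross is centered on X and shifted in Z by Offset, leaving the computed CenterZ unused.
; Its event graph is empty.
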(event EventBeginPlay)

(event Collision|EventActorBeginOverlap
  (params (OtherActor :type Actor%20Object%20Reference)))

(event EventTick
  (params (DeltaSeconds :type Float%20%28single-precision%29)))

(fn ConstructionScript
  (bind _stones_xz (Variables|Default|GetStones%20XZ))
  (bind _cube (Variables|Default|Getcube))
  (bind _stones_xz_2 (Variables|Default|GetStones%20XZ))
  (bind (_min _max) (Components|StaticMesh|GetLocalBounds _cube))
  (bind _returnvalue (- _stones_xz_2 1))
  (bind _returnvalue_2 (- _stones_xz 1))
  (bind _returnvalue_3 (Math|Conversions|ToFloat(Integer) _returnvalue))
  ;[1 1 1] set static mesh et material
  (Components|StaticMesh|SetStaticMesh (Variables|Default|Getcube) (Variables|Default|GetSM_Stone))
  (LocalVariables|Setcenter (- _max _min))
  (LocalVariables|SetcenterX (* _returnvalue_3 (/ (.x (LocalVariables|Getcenter)) 2.0)))
  (LocalVariables|SetCenterZ (* _returnvalue_3 (/ (.z (LocalVariables|Getcenter)) 2.0)))
  (for _index (range 0 _returnvalue_2)
    (LocalVariables|SetX _index)
    (for _index_2 (range 0 _returnvalue_2)
      (LocalVariables|SetZIndex%20 _index_2)
      (if (or (== (LocalVariables|GetX) (LocalVariables|GetZIndex%20)) (== (LocalVariables|GetX) (- (- (Variables|Default|GetStones%20XZ) 1) (LocalVariables|GetZIndex%20))))
        (Components|InstancedStaticMesh|AddInstance (Variables|Default|Getcube) (Math|Transform|MakeTransform (Math|Vector|MakeVector (- (* (Math|Conversions|ToFloat(Integer) (LocalVariables|GetX)) (.x (LocalVariables|Getcenter))) (LocalVariables|GetcenterX)) 0.0 (+ (* (Math|Conversions|ToFloat(Integer) (LocalVariables|GetZIndex%20)) (.z (LocalVariables|Getcenter))) (Variables|Default|GetOffset)))) false)))))