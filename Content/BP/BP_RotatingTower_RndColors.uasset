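; Construction-script actor that builds a twisting tower of stacked mesh instances, each with a random color.
; It validates mesh, material and count, logging on failure, then clears and rebuilds the Cube instanced mesh component.
; Instances stack by mesh bounds height and rotate progressively through a full turn.
; Random RGB goes into three per-instance custom data floats for the material, avoiding separate materials per block.
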(event EventBeginPlay)

(event Collision|EventActorBeginOverlap
  (params (OtherActor :type Actor%20Object%20Reference)))

(event EventTick
  (params (DeltaSeconds :type Float%20%28single-precision%29)))

(fn ConstructionScript
  (bind _cube (Variables|Default|Getcube))
  (bind _cube_2 (Variables|Default|Getcube))
  (bind (_min _max) (Components|StaticMesh|GetLocalBounds _cube_2))
  (if (Math|Boolean|ORBoolean (== (Variables|Default|GetMaterial) 0) (== (Variables|Default|GetSM_Stone) 0) (< (Variables|Default|GetNombre%20De%20cube) 1))
    (Utilities|String|LogString "Null value ")
    (else
      (Components|InstancedStaticMesh|ClearInstances (Variables|Default|Getcube))
      ;[1 1 1] set static mesh et material
      (Components|StaticMesh|SetStaticMesh (Variables|Default|Getcube) (Variables|Default|GetSM_Stone))
      (Rendering|Material|SetMaterial (Variables|Default|Getcube) 0 (Variables|Default|GetMaterial))
      (LocalVariables|Setcenter (- _max _min))
      (Class|InstancedStaticMeshComponent|SetNumCustomDataFloats (Variables|Default|Getcube) 3)
      (LocalVariables|Setangle%20step (/ 3.6e+02 (Math|Conversions|ToFloat(Integer) (- (Variables|Default|GetNombre%20De%20cube) 1))))
      (for _index (range 0 (- (Variables|Default|GetNombre%20De%20cube) 1))
        (bind _output_get (LocalVariables|Seti _index))
        (LocalVariables|Setangle (* (Math|Conversions|ToFloat(Integer) _output_get) (LocalVariables|Getangle%20step)))
        (LocalVariables|SetR (Math|Random|RandomFloatinRange 0.0 1.0))
        (LocalVariables|SetG (Math|Random|RandomFloatinRange 0.0 1.0))
        (LocalVariables|SetB (Math|Random|RandomFloatinRange 0.0 1.0))
        (LocalVariables|SetPos (Math|Vector|MakeVector 0.0 0.0 (* (.z (LocalVariables|Getcenter)) (LocalVariables|Geti))))
        (LocalVariables|SetRot (Math|Rotator|MakeRotator 0.0 0.0 (LocalVariables|Getangle)))
        (Components|InstancedStaticMesh|AddInstance (Variables|Default|Getcube) (Math|Transform|MakeTransform (LocalVariables|GetPos) (LocalVariables|GetRot)) false)
        (Components|InstancedStaticMesh|SetCustomDataValue _cube (LocalVariables|Geti) 0 (LocalVariables|GetR) false)
        (Components|InstancedStaticMesh|SetCustomDataValue _cube (LocalVariables|Geti) 1 (LocalVariables|GetG) false)
        (Components|InstancedStaticMesh|SetCustomDataValue _cube (LocalVariables|Geti) 2 (LocalVariables|GetB) false)))))