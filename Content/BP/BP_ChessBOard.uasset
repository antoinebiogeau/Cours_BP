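; BP_ChessBOard procedurally builds an upright checkerboard in the XZ plane from instanced stone meshes.
; Its construction script sets the mesh and material, then loops over X by Y cells, spacing instances by mesh bounds.
; Cell parity writes three per-instance custom data floats as all ones or default values, letting one material distinguish alternating squares.
; The event graph has no active logic.
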(event EventBeginPlay)

(event Collision|EventActorBeginOverlap
  (params (OtherActor :type Actor%20Object%20Reference)))

(event EventTick
  (params (DeltaSeconds :type Float%20%28single-precision%29)))

(fn ConstructionScript
  (bind _cube (Variables|Default|Getcube))
  (bind (_min _max) (Components|StaticMesh|GetLocalBounds _cube))
  (Class|InstancedStaticMeshComponent|SetNumCustomDataFloats (Variables|Default|Getcube) 3)
  ;[1 1 1] set static mesh et material
  (Components|StaticMesh|SetStaticMesh (Variables|Default|Getcube) (Variables|Default|GetSM_Stone))
  (Rendering|Material|SetMaterial (Variables|Default|Getcube) 0 (Variables|Default|GetMaterial))
  (LocalVariables|Setcenter (- _max _min))
  (for _index (range 0 (- (Variables|Default|GetX) 1))
    (LocalVariables|Seti _index)
    (for _index_2 (range 0 (- (Variables|Default|GetY) 1))
      (LocalVariables|Setj _index_2)
      (bind _returnvalue (Components|InstancedStaticMesh|AddInstance (Variables|Default|Getcube) (Math|Transform|MakeTransform (Math|Vector|MakeVector (* (.x (LocalVariables|Getcenter)) (LocalVariables|Geti)) 0.0 (+ (* (.z (LocalVariables|Getcenter)) (LocalVariables|Getj)) 5e+01)) "0, 0, 0" "1.000000,1.000000,1.000000") false))
      (LocalVariables|Setindex%20instance _returnvalue)
      (if (== (Math|Integer|%(Integer) (+ (LocalVariables|Geti) (LocalVariables|Getj)) 2) 0)
        ;[1 1 1] custom data
        (Components|InstancedStaticMesh|SetCustomDataValue (Variables|Default|Getcube) (LocalVariables|Getindex%20instance) 0 1.0 false)
        (Components|InstancedStaticMesh|SetCustomDataValue (Variables|Default|Getcube) (LocalVariables|Getindex%20instance) 1 1.0 false)
        (Components|InstancedStaticMesh|SetCustomDataValue (Variables|Default|Getcube) (LocalVariables|Getindex%20instance) 2 1.0 false)
        (else
          (Components|InstancedStaticMesh|SetCustomDataValue (Variables|Default|Getcube) (LocalVariables|Getindex%20instance) 0 0.0 false)
          (Components|InstancedStaticMesh|SetCustomDataValue (Variables|Default|Getcube) (LocalVariables|Getindex%20instance) 1 0.0 false)
          (Components|InstancedStaticMesh|SetCustomDataValue (Variables|Default|Getcube) (LocalVariables|Getindex%20instance) 2 0.0 false))))))