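; Construction-script Blueprint that builds a hollow cube frame from instances of a configurable stone mesh.
; Nested loops over the StoneX, StoneY and StoneZ counts add instances only where two axes are at their limits, leaving just the box edges.
; Mesh bounds drive X/Y centering, but X width spaces both axes; Z uses a fixed 100-unit step plus Offset.
; The event graph is unused.
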(event EventBeginPlay)

(event Collision|EventActorBeginOverlap
  (params (OtherActor :type Actor%20Object%20Reference)))

(event EventTick
  (params (DeltaSeconds :type Float%20%28single-precision%29)))

(fn ConstructionScript
  (bind _cube (Variables|Default|Getcube))
  (bind (_min _max) (Components|StaticMesh|GetLocalBounds _cube))
  ;[1 1 1] set static mesh et material
  (Components|StaticMesh|SetStaticMesh (Variables|Default|Getcube) (Variables|Default|GetSM_Stone))
  (bind _output_get (LocalVariables|Setcenter (- _max _min)))
  (LocalVariables|SetCenterOffsetX (* (- (Variables|Default|GetStoneX) 1.0) (/ (.x _output_get) 2.0)))
  (LocalVariables|SetCenterOffsetY (* (- (Variables|Default|GetStoneY) 1) (/ (.y _output_get) 2.0)))
  (for _index (range 0 (- (Variables|Default|GetStoneZ) 1))
    (LocalVariables|SetZ _index)
    (for _index_2 (range 0 (- (Variables|Default|GetStoneY) 1))
      (LocalVariables|SetY _index_2)
      (for _index_3 (range 0 (- (Variables|Default|GetStoneX) 1))
        (LocalVariables|SetX _index_3)
        (if (Math|Boolean|ORBoolean (and (or (== (LocalVariables|GetX) 0) (== (LocalVariables|GetX) (- (Variables|Default|GetStoneX) 1))) (or (== (LocalVariables|GetY) 0) (== (LocalVariables|GetY) (- (Variables|Default|GetStoneY) 1)))) (and (or (== (LocalVariables|GetX) 0) (== (LocalVariables|GetX) (- (Variables|Default|GetStoneX) 1))) (or (== (LocalVariables|GetZ) 0) (== (LocalVariables|GetZ) (- (Variables|Default|GetStoneZ) 1)))) (and (or (== (LocalVariables|GetY) 0) (== (LocalVariables|GetY) (- (Variables|Default|GetStoneY) 1))) (or (== (LocalVariables|GetZ) 0) (== (LocalVariables|GetZ) (- (Variables|Default|GetStoneZ) 1)))))
          (Components|InstancedStaticMesh|AddInstance (Variables|Default|Getcube) (Math|Transform|MakeTransform (Math|Vector|MakeVector (- (* (.x (LocalVariables|Getcenter)) (LocalVariables|GetX)) (LocalVariables|GetCenterOffsetX)) (- (* (.x (LocalVariables|Getcenter)) (LocalVariables|GetY)) (LocalVariables|GetCenterOffsetY)) (- (* (LocalVariables|GetZ) 1e+02) (- 0.0 (Variables|Default|GetOffset)))) "0, 0, 0" "1.000000,1.000000,1.000000") false))))))