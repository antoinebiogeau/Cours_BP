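; BP_CubesInSphereRadius is an actor, named for cubes within a sphere radius, that prepares an instanced static mesh component in its Construction Script.
; It logs "Null value" if material, mesh or cube count is invalid; otherwise it clears instances and applies mesh and material.
; It stores the bounds size in Center and reserves three custom data floats per instance.
; No instances are placed yet, and the event graph is empty.
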(event EventBeginPlay)

(event Collision|EventActorBeginOverlap
  (params (OtherActor :type Actor%20Object%20Reference)))

(event EventTick
  (params (DeltaSeconds :type Float%20%28single-precision%29)))

(fn ConstructionScript
  (bind _cube (LocalVariables|Getcube))
  (bind (_min _max) (Components|StaticMesh|GetLocalBounds _cube))
  (if (Math|Boolean|ORBoolean (== (Variables|Default|GetMaterial) 0) (== (Variables|Default|GetSM_Stone) 0) (< (Variables|Default|GetNombre%20De%20cube) 1))
    (Utilities|String|LogString "Null value ")
    (else
      (Components|InstancedStaticMesh|ClearInstances (LocalVariables|Getcube))
      ;[1 1 1] set static mesh et material
      (Components|StaticMesh|SetStaticMesh (LocalVariables|Getcube) (Variables|Default|GetSM_Stone))
      (Rendering|Material|SetMaterial (LocalVariables|Getcube) 0 (Variables|Default|GetMaterial))
      (LocalVariables|Setcenter (- _max _min))
      (Class|InstancedStaticMeshComponent|SetNumCustomDataFloats (LocalVariables|Getcube) 3))))