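; Construction-script actor that builds an upright checkerboard of stone mesh instances in the XZ plane, leaving alternate cells empty.
; It assigns the stone mesh to an instanced mesh component and uses that mesh's local bounds as grid spacing.
; Nested loops over X columns and Y rows add an instance only where the index sum is even, raised by a fixed Z offset.
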(event EventBeginPlay)

(event Collision|EventActorBeginOverlap
  (params (OtherActor :type Actor%20Object%20Reference)))

(event EventTick
  (params (DeltaSeconds :type Float%20%28single-precision%29)))

(fn ConstructionScript
  (bind _cube (Variables|Default|Getcube))
  (bind (_min _max) (Components|StaticMesh|GetLocalBounds _cube))
  ;[1 1 1] set static mesh et material
  (Components|StaticMesh|SetStaticMesh (Variables|Default|Getcube) (Variables|Default|GetSM_Stone))
  (LocalVariables|Setcenter (- _max _min))
  (for _index (range 0 (- (Variables|Default|GetX) 1))
    (LocalVariables|Seti _index)
    (for _index_2 (range 0 (- (Variables|Default|GetY) 1))
      (LocalVariables|Setj _index_2)
      (if (== (Math|Integer|%(Integer) (+ (LocalVariables|Geti) (LocalVariables|Getj)) 2) 0)
        (Components|InstancedStaticMesh|AddInstance (Variables|Default|Getcube) (Math|Transform|MakeTransform (Math|Vector|MakeVector (* (.x (LocalVariables|Getcenter)) (LocalVariables|Geti)) 0.0 (+ (* (.z (LocalVariables|Getcenter)) (LocalVariables|Getj)) 5e+01)) "0, 0, 0" "1.000000,1.000000,1.000000") false)))))