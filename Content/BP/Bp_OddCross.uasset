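; Blueprint actor that builds a cross of stone mesh instances in its construction script, with no active event logic.
; It rounds StoneX and StoneZ up to odd counts and uses mesh bounds to space and center the horizontal row at mid-height.
; The vertical column loop is nested inside the row loop and counts by StoneXODD rather than StoneZODD, so column instances are duplicated on each pass.
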(event EventBeginPlay)

(event Collision|EventActorBeginOverlap
  (params (OtherActor :type Actor%20Object%20Reference)))

(event EventTick
  (params (DeltaSeconds :type Float%20%28single-precision%29)))

(fn ConstructionScript
  (bind _cube (Variables|Default|Getcube))
  (bind (_min _max) (Components|StaticMesh|GetLocalBounds _cube))
  ;[1 1 1] set static mesh et material
  (Components|StaticMesh|SetStaticMesh (Variables|Default|Getcube) (Variables|Default|GetSM_Stone))
  (bind _output_get (LocalVariables|Setcenter (- _max _min)))
  (LocalVariables|SetCenterOffsetX (* (- (Variables|Default|GetStoneX) 0.0) (.x _output_get)))
  (LocalVariables|SetCenterOffsetY (* (- 0 1) (.y _output_get)))
  (if (== (Math|Integer|%(Integer) (Variables|Default|GetStoneX) 2) 0)
    (LocalVariables|SetStoneXODD (+ (Variables|Default|GetStoneX) 1))
    (else
      (LocalVariables|SetStoneXODD (Variables|Default|GetStoneX))))
  (if (== (Math|Integer|%(Integer) (Variables|Default|GetStoneZ) 2) 0)
    (LocalVariables|SetStoneZODD (+ (Variables|Default|GetStoneZ) 1))
    (else
      (LocalVariables|SetStoneZODD (Variables|Default|GetStoneZ))))
  (LocalVariables|SetCenterOffsetX%20 (/ (* (- (LocalVariables|GetStoneXODD) 1) (.x (LocalVariables|Getcenter))) 2.0))
  (bind _output_get_2 (LocalVariables|SetCenterOffsetZ%20 (/ (* (- (LocalVariables|GetCenterOffsetZ%20) 1) (.z (LocalVariables|Getcenter))) 2.0)))
  (LocalVariables|SetZfixed _output_get_2)
  (for _index (range 0 (- (LocalVariables|GetStoneXODD) 1))
    (LocalVariables|SetX _index)
    (bind _output_get_3 (LocalVariables|Setloc (Math|Vector|MakeVector (- (* (LocalVariables|GetX) (.x (LocalVariables|Getcenter))) (LocalVariables|GetCenterOffsetX%20)) 0.0 (+ (+ (LocalVariables|GetZfixed) (Variables|Default|GetOffset)) (* (.z (LocalVariables|Getcenter)) (/ (LocalVariables|GetStoneZODD) 2))))))
    (Components|InstancedStaticMesh|AddInstance (Variables|Default|Getcube) (Math|Transform|MakeTransform _output_get_3 "0, 0, 0" "1.000000,1.000000,1.000000") false)
    (for _index_2 (range 0 (- (LocalVariables|GetStoneXODD) 1))
      (LocalVariables|SetZ _index_2)
      (Components|InstancedStaticMesh|AddInstance (Variables|Default|Getcube) (Math|Transform|MakeTransform (Math|Vector|MakeVector 0.0 0.0 (+ (* (LocalVariables|GetZ) (.z (LocalVariables|Getcenter))) (Variables|Default|GetOffset))) "0, 0, 0" "1.000000,1.000000,1.000000") false))))