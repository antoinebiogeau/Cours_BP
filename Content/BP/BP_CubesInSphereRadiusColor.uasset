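; Construction-script actor that scatters instanced mesh cubes at random directions and distances around its origin within a radius.
; Rebuilds the Cube instances from the chosen mesh and material, using the outer scale near the radius edge and the inner scale elsewhere, with look-at rotations toward the center.
; Writes three random custom data floats per instance, likely color for the material.
; Seeds a random stream, but the random calls do not use it.
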(event EventBeginPlay)

(event Collision|EventActorBeginOverlap
  (params (OtherActor :type Actor%20Object%20Reference)))

(event EventTick
  (params (DeltaSeconds :type Float%20%28single-precision%29)))

(fn ConstructionScript
  (bind _returnvalue (Math|Random|RandomFloatinRange 0.0 1.0))
  (bind _returnvalue_2 (Math|Vector|VectorZero))
  (bind _returnvalue_3 (Math|Vector|VectorZero))
  (bind _cube (Variables|Default|Getcube))
  (bind _cube_2 (Variables|Default|Getcube))
  (bind (_min _max) (Components|StaticMesh|GetLocalBounds _cube))
  (bind _returnvalue_4 (- _max _min))
  (Math|Random|SetRandomStreamSeed (LocalVariables|GetNewLocalVar_0) (LocalVariables|GetNewLocalVar_1))
  (if (Math|Boolean|ORBoolean (== (Variables|Default|GetMaterial) 0) (== (Variables|Default|GetSM_Stone) 0) (< (Variables|Default|GetNombre%20De%20cube) 1))
    (Utilities|String|LogString "Null value ")
    (else
      (Components|InstancedStaticMesh|ClearInstances (Variables|Default|Getcube))
      ;[1 1 1] set static mesh et material
      (Components|StaticMesh|SetStaticMesh _cube_2 (Variables|Default|GetSM_Stone))
      (Rendering|Material|SetMaterial _cube_2 0 (Variables|Default|GetMaterial))
      (LocalVariables|Setcenter _returnvalue_4)
      (LocalVariables|SetHalfCube (/ _returnvalue_4 (LocalVariables|GetNewLocalVar)))
      (Class|InstancedStaticMeshComponent|SetNumCustomDataFloats (Variables|Default|Getcube) 3)
      (for _index (range 0 (- (Variables|Default|GetNombre%20De%20cube) 1))
        (bind _output_get (LocalVariables|SetD (Math|Random|RandomFloatinRange 0.0 (Variables|Default|GetRadius))))
        (if (>= _output_get (* (Variables|Default|GetRadius) (- 1.0 (Variables|Default|GetError%20Tolerance))))
          (bind _returnvalue_5 (Components|InstancedStaticMesh|AddInstance (Variables|Default|Getcube) (Math|Transform|MakeTransform (+ _returnvalue_3 (* (Math|Random|RandomUnitVector) (+ (LocalVariables|GetD) (* (.x (LocalVariables|GetHalfCube)) (.x (Variables|Default|GetOuterScale)))))) (Math|Rotator|FindLookatRotation (+ _returnvalue_3 (* (Math|Random|RandomUnitVector) (+ (LocalVariables|GetD) (* (.x (LocalVariables|GetHalfCube)) (.x (Variables|Default|GetOuterScale)))))) _returnvalue_3) (Variables|Default|GetOuterScale)) false))
          (Components|InstancedStaticMesh|SetCustomDataValue (Variables|Default|Getcube) _returnvalue_5 0 _returnvalue false)
          (Components|InstancedStaticMesh|SetCustomDataValue (Variables|Default|Getcube) _returnvalue_5 1 _returnvalue false)
          (Components|InstancedStaticMesh|SetCustomDataValue (Variables|Default|Getcube) _returnvalue_5 2 _returnvalue false)
          (else
            (bind _returnvalue_6 (Components|InstancedStaticMesh|AddInstance (Variables|Default|Getcube) (Math|Transform|MakeTransform (+ _returnvalue_2 (* (Math|Random|RandomUnitVector) (+ (LocalVariables|GetD) (* (.x (LocalVariables|GetHalfCube)) (.x (Variables|Default|GetInner%20scale)))))) (Math|Rotator|FindLookatRotation (+ _returnvalue_2 (* (Math|Random|RandomUnitVector) (+ (LocalVariables|GetD) (* (.x (LocalVariables|GetHalfCube)) (.x (Variables|Default|GetInner%20scale)))))) _returnvalue_2) (Variables|Default|GetInner%20scale)) false))
            (Components|InstancedStaticMesh|SetCustomDataValue (Variables|Default|Getcube) _returnvalue_6 0 _returnvalue false)
            (Components|InstancedStaticMesh|SetCustomDataValue (Variables|Default|Getcube) _returnvalue_6 1 _returnvalue false)
            (Components|InstancedStaticMesh|SetCustomDataValue (Variables|Default|Getcube) _returnvalue_6 2 _returnvalue false)))))))